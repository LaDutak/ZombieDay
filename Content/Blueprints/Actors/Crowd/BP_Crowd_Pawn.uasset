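; Crowd pawn that advances a fixed step along a spline on cursor clicks and opens First_Level shortly after overlapping a BP_Zombie_1.
; Tick polls FollowMouse, briefly shows the R circle effect, and uses a counter to turn a held press into a single step.
; Each step moves the Cube crowd mesh and R to the new spline transform, then stores the crowd's relative position in LocationOfCrowd.
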(event `CustomEvent`
  (bind _r (`self.r`))
  ;[1 1 1] Эффект круга
  (`SceneComponent.SetHiddenInGame` _r false false)
  (`KismetSystemLibrary.Delay` 1.0)
  (`SceneComponent.SetHiddenInGame` _r true false))

(event `self.ReceiveTick`
  (params (DeltaSeconds :type "Float (single-precision)"))
  (bind _r (`self.r`))
  (bind _cube (`self.Cube`))
  (bind (_returnvalue_location _returnvalue_rotation) (`KismetMathLibrary.BreakTransform` (`SplineComponent.GetTransformAtDistanceAlongSpline` (`self.Spline`) (`self.Distance`) "Local" false)))
  ;[1 1 1] Клик курсором
  (if (`self.FollowMouse`)
    (`self.CustomEvent`) ; Эффект круга
    (bind _output_get (set `self.Counter` (+ (`self.Counter`) 1)))
    (if (> _output_get 1)
      (set `self.FollowMouse` false)
      (set `self.Counter` 0)
      ;[1 1 1] Перемещение по сплайну
      (set `self.Distance` (+ (`self.Distance`) 30.0))
      (`SceneComponent.K2_SetRelativeTransform` _cube (`KismetMathLibrary.MakeTransform` _returnvalue_location _returnvalue_rotation (`SceneComponent.RelativeScale3D` _cube)) false false) ; толпа
      (`SceneComponent.K2_SetRelativeTransform` _r (`KismetMathLibrary.MakeTransform` _returnvalue_location _returnvalue_rotation (`SceneComponent.RelativeScale3D` _r)) false false) ; эффект
      (set `self.Location of Crowd` (`SceneComponent.RelativeLocation` (`self.Cube`))))))

(event `self.ReceiveActorBeginOverlap`
  (params (OtherActor :type "Actor Object Reference"))
  ;[1 1 1] Столкновение с зомби
  (cast `/Game/Blueprints/Actors/Zombie/BP_Zombie_1` OtherActor)
  (`KismetSystemLibrary.Delay` 1.0)
  (`GameplayStatics.OpenLevel` "First_Level"))

(fn `UserConstructionScript`)