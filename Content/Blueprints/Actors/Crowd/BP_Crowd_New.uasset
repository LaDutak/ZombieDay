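; Crowd actor that advances along a spline after being clicked and costs the player HP when zombies reach it.
; While FollowMouse is set, Tick flags the controller's first touch, flashes Niagara and moves mesh and collision box by the GameInstance's distance bonus per frame.
; A two-second timer clears FollowMouse to end movement.
; Overlapping zombies not following the mouse deduct HP after a short delay, then are destroyed.
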(event `NiagaraEvent`
  (bind _niagara (`self.Niagara`))
  ;[1 1 1] Niagara
  (`SceneComponent.SetHiddenInGame` _niagara false false)
  (`AddComponent|NODE_AddNiagaraComponent-4` :`self` (`ActorComponent.GetOwner` _niagara))
  (`KismetSystemLibrary.Delay` 1.0)
  (`SceneComponent.SetHiddenInGame` _niagara true false))

(event `GO!`)

(event `self.ReceiveTick`
  (params (DeltaSeconds :type "Float (single-precision)"))
  (bind _box (`self.Box`))
  (bind _cube1 (`self.Cube1`))
  (bind (_returnvalue_location _returnvalue_rotation) (`KismetMathLibrary.BreakTransform` (`SplineComponent.GetTransformAtDistanceAlongSpline` (`self.Spline`) (`self.Distance`) "Local" false)))
  ;[1 1 1] Клик курсором
  (if (`self.FollowMouse`)
    (`self.NiagaraEvent`)
    (bind _asmy_player_controller (cast `/Game/Blueprints/AllCharacter/MyPlayerController` (`GameplayStatics.GetPlayerController` 0)))
    (set `/Game/Blueprints/AllCharacter/MyPlayerController.WasTouch?` true _asmy_player_controller) ; игра не начнется, пока не нажмем по толпе
    (bind _output_get (set `self.Counter` (+ (`self.Counter`) 1)))
    (if (> _output_get 1)
      (set `self.Don't Touch` true) ; начинается джижение
      (bind _output_get_2 (set `self.Timer` (+ (`self.Timer`) DeltaSeconds)))
      (if (>= _output_get_2 2.0)
        (set `self.Timer` 0.0)
        (set `self.Don't Touch` false) ; начинается джижение
        (set `self.FollowMouse` false)
        (else
          ;[1 1 1] Перемещение по сплайну
          (bind _asmy_game_instance (cast `/Game/Blueprints/AllCharacter/MyGameInstance` (`GameplayStatics.GetGameInstance`)))
          (set `self.Distance` (+ (`self.Distance`) (`/Game/Blueprints/AllCharacter/MyGameInstance.DistanceBonus` _asmy_game_instance)))
          (`SceneComponent.K2_SetRelativeTransform` _cube1 (`KismetMathLibrary.MakeTransform` _returnvalue_location _returnvalue_rotation (`SceneComponent.RelativeScale3D` _cube1)) false false) ; толпа
          (`SceneComponent.K2_SetRelativeTransform` _box (`KismetMathLibrary.MakeTransform` _returnvalue_location _returnvalue_rotation (`SceneComponent.RelativeScale3D` _box)) false false) ; collision
          (set `self.Location of Crowd` (`SceneComponent.RelativeLocation` (`self.Box`))))))))

(event `self.ReceiveActorBeginOverlap`
  (params (OtherActor :type "Actor Object Reference"))
  ;[0.4072 0.4072 0.4072] Столкновение с зомби
  (bind _asbp_zombie_1 (cast `/Game/Blueprints/Actors/Zombie/BP_Zombie_1` OtherActor))
  (if (not (`/Game/Blueprints/Actors/Zombie/BP_Zombie_1.FollowMouse` _asbp_zombie_1))
    (`KismetSystemLibrary.Delay` 0.3)
    (bind _asmy_player_controller (cast `/Game/Blueprints/AllCharacter/MyPlayerController` (`GameplayStatics.GetPlayerController` 0)))
    (set `/Game/Blueprints/AllCharacter/MyPlayerController.HP` (- (`/Game/Blueprints/AllCharacter/MyPlayerController.HP` _asmy_player_controller) 1) _asmy_player_controller)
    (`self.K2_DestroyActor` _asbp_zombie_1)))

(fn `UserConstructionScript`)