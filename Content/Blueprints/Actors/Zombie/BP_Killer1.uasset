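; BP_Killer1 is a zone actor that destroys a BP_Zombie_1 when it overlaps the actor.
; Each Tick it looks up a BP_Zombie_1 and switches its plane to an arrow material while that zombie follows the mouse, otherwise to an earth material.
; On a kill it sets Killed, clears Spawned on its Collision reference, and clears the player controller's Stop flag when LevelBP is 1.
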(event `self.ReceiveTick`
  (params (DeltaSeconds :type "Float (single-precision)"))
  (bind _plane (`self.Plane`))
  ;[1 1 1] Смена материала
  (bind _returnvalue (`GameplayStatics.GetActorOfClass` "/Game/Blueprints/Actors/Zombie/BP_Zombie_1.BP_Zombie_1_C"))
  (`/Engine/EditorBlueprintResources/StandardMacros.IsValid` _returnvalue
    (:`Is Valid`
      (if (`/Game/Blueprints/Actors/Zombie/BP_Zombie_1.FollowMouse` _returnvalue)
        (`PrimitiveComponent.SetMaterial` _plane 0 "/Game/Art/Materials/MI_ArrowZ.MI_ArrowZ")
        (else
          (`PrimitiveComponent.SetMaterial` _plane 0 "/Game/Art/Prototype/MM_Earth.MM_Earth" :!label _label))))
    (:`Is Not Valid`
      (goto _label))))

(event `self.ReceiveActorBeginOverlap`
  (params (OtherActor :type "Actor Object Reference"))
  (bind _collision (`self.Collision`))
  ;[1 1 1] Убийство зомби
  (bind _asbp_zombie_1 (cast `/Game/Blueprints/Actors/Zombie/BP_Zombie_1` OtherActor))
  (bind _asmy_player_controller (cast `/Game/Blueprints/AllCharacter/MyPlayerController` (`GameplayStatics.GetPlayerController` 0)))
  (if (== (`/Game/Blueprints/AllCharacter/MyPlayerController.LevelBP` _asmy_player_controller) 1)
    (set `/Game/Blueprints/AllCharacter/MyPlayerController.Stop` false _asmy_player_controller))
  (set `self.Killed` true)
  (`self.K2_DestroyActor` _asbp_zombie_1)
  (`/Engine/EditorBlueprintResources/StandardMacros.IsValid` _collision
    (:`Is Valid`
      (set `/Game/Blueprints/Actors/Other/BP_CollisionSpawn.Spawned` false _collision))))

(fn `UserConstructionScript`)