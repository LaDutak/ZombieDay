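; Zombie actor that uses AI movement to head for the crowd actor, with an option to follow the mouse cursor.
; Every Tick it reissues AI MoveTo toward an actor found by CrowdRef's class.
; When FollowMouse is set, it also shows its Plane and snaps to the cursor's visibility-trace hit; otherwise the Plane is hidden.
; The Follow event is empty, and the sight and debug-print nodes are disconnected leftovers.
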(event `self.ReceiveBeginPlay`)

(event `self.ReceiveTick`
  (params (DeltaSeconds :type "Float (single-precision)"))
  (bind _plane (`self.Plane`))
  (bind _returnvalue (`GameplayStatics.GetActorOfClass` (`GameplayStatics.GetObjectClass` (`self.Crowd_Ref`))))
  (`|AIMoveTo` self (0.0 0.0 0.0) _returnvalue 1.0
    (:`then`
      (if (`self.FollowMouse`)
        ;[1 1 1] перемещение под курсором
        (`SceneComponent.SetHiddenInGame` _plane false false)
        (`self.K2_SetActorLocation` (`.Location` (`GameplayStatics.BreakHitResult` (`PlayerController.GetHitResultUnderCursorByChannel` (`GameplayStatics.GetPlayerController` 0) "TraceTypeQuery1" true))))
        (else
          (`SceneComponent.SetHiddenInGame` _plane true false))))))

(event `Follow`
  ;[1 1 1] AI
)

(fn `UserConstructionScript`)