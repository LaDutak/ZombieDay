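; BP_Zombie_2 is a zombie pawn that can be positioned with the mouse and sent toward a crowd.
; While FollowMouse is set, Tick shows its Plane and snaps it to the cursor trace hit, clamping height; otherwise the Plane is hidden.
; The GO! event runs AI MoveTo toward Cube1 on CrowdRef and destroys the zombie on success.
; The overlap event is empty; HP damage and level-check logic are disconnected.
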(event `self.ReceiveTick`
  (params (DeltaSeconds :type "Float (single-precision)"))
  (bind _plane (`self.Plane`))
  (bind (_bblockinghit _binitialoverlap _time _distance _location) (`GameplayStatics.BreakHitResult` (`PlayerController.GetHitResultUnderCursorByChannel` (`GameplayStatics.GetPlayerController` 0) "TraceTypeQuery1" true)))
  ;[1 1 1] перемещение под курсором
  (if (`self.FollowMouse`)
    (`SceneComponent.SetHiddenInGame` _plane false false)
    (`self.K2_SetActorLocation` (`KismetMathLibrary.MakeVector` (.x _location) (.y _location) (`KismetMathLibrary.Conv_IntToDouble` (`KismetMathLibrary.Clamp` (`KismetMathLibrary.FTrunc` (.z _location)) 0 200))))
    (else
      (`SceneComponent.SetHiddenInGame` _plane true false))))

(event `GO!`
  ;[0.07701 0.8319 1] AI
  (`|AIMoveTo` self (`SceneComponent.K2_GetComponentLocation` (`/Game/Blueprints/Actors/Crowd/BP_Crowd_New.Cube1` (`self.Crowd_Ref`))) null
    (:`OnSuccess`
      (`self.K2_DestroyActor`))))

(event `self.ReceiveActorBeginOverlap`
  (params (OtherActor :type "Actor Object Reference"))
  ;[0.07701 0.8319 1] Столкновение с толпой
)

(fn `UserConstructionScript`)