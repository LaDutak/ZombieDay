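; BP_Spawner is a zombie spawner actor built around BP_Zombie_1.
; Tick runs a five-second timer, then raises an anti-collision protection flag and looks up an existing zombie.
; An unnamed custom event, not called here, spawns a zombie above the spawner with that zombie's CrowdRef, resets the timer and clears the flag after a delay.
; The overlap event is empty, leaving the flag-gated self-destroy logic disconnected.
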(event `self.ReceiveActorBeginOverlap`
  (params (OtherActor :type "Actor Object Reference"))
  ;[1 1 1] Уничтожение зомби
)

(event `CustomEvent`
  (bind (_returnvalue_x _returnvalue_y _returnvalue_z) (`KismetMathLibrary.BreakVector` (`SceneComponent.K2_GetComponentLocation` (`self.DefaultSceneRoot`))))
  ;[1 1 1] Спавн
  (`|SpawnActorFromClass` "/Game/Blueprints/Actors/Zombie/BP_Zombie_1.BP_Zombie_1_C" (`KismetMathLibrary.MakeTransform` (`KismetMathLibrary.MakeVector` _returnvalue_x _returnvalue_y (+ _returnvalue_z 200.0))) "Undefined" "MultiplyWithRoot" null (`/Game/Blueprints/Actors/Zombie/BP_Zombie_1.Crowd_Ref` (stale `self.ReceiveTick` _returnvalue)) null) ; спавн
  (`KismetSystemLibrary.PrintString` "Hello")
  (set `self.Timer` 0.0)
  (`KismetSystemLibrary.Delay` 3.0)
  (set `self.Undestoyadle?` false))

(event `self.ReceiveTick`
  (params (DeltaSeconds :type "Float (single-precision)"))
  ;[1 1 1] Спавн
  (bind _output_get (set `self.Timer` (+ DeltaSeconds (`self.Timer`))))
  (if (>= _output_get 5.0)
    (set `self.Undestoyadle?` true) ; защита от коллизии
    (bind _returnvalue (`GameplayStatics.GetActorOfClass` "/Game/Blueprints/Actors/Zombie/BP_Zombie_1.BP_Zombie_1_C"))))

(fn `UserConstructionScript`)