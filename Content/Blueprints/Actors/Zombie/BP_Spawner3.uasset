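; BP_Spawner3 is a zombie spawner actor whose only live logic is a custom event, noted as a first-level workaround.
; After a short delay, it shows an arrow material on its plane and spawns BP_Zombie_1 above itself.
; After another delay, it clears Undestoyadle and switches the plane to the earth material.
; Overlap and Tick are empty; self-destruction and timed, touch-gated spawning for other levels are disconnected.
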(event `self.ReceiveActorBeginOverlap`
  (params (OtherActor :type "Actor Object Reference"))
  ;[1 1 1] Уничтожение зомби
)

(event `CustomEvent`
  (bind _plane (`self.Plane`))
  (bind (_returnvalue_x _returnvalue_y _returnvalue_z) (`KismetMathLibrary.BreakVector` (`SceneComponent.K2_GetComponentLocation` (`self.DefaultSceneRoot`))))
  ;[1 1 1] Костыль для первого уровня
  (`KismetSystemLibrary.Delay` 1.0)
  (`PrimitiveComponent.SetMaterial` _plane 0 "/Game/Art/Materials/MM_Arrow.MM_Arrow")
  (`|SpawnActorFromClass` "/Game/Blueprints/Actors/Zombie/BP_Zombie_1.BP_Zombie_1_C" (`KismetMathLibrary.MakeTransform` (`KismetMathLibrary.MakeVector` _returnvalue_x _returnvalue_y (+ _returnvalue_z 200.0))) "Undefined" "MultiplyWithRoot" null null null) ; спавн
  (`KismetSystemLibrary.PrintString` "Hello")
  (set `self.Timer` 0.0)
  (`KismetSystemLibrary.Delay` 3.0)
  (set `self.Undestoyadle?` false)
  (`PrimitiveComponent.SetMaterial` _plane 0 "/Game/Art/Prototype/MM_Earth.MM_Earth"))

(event `self.ReceiveTick`
  (params (DeltaSeconds :type "Float (single-precision)"))
  ;[1 1 1] Спавн
  ;;[1 1 1] Проверка: не первый ли уровень?
)

(fn `UserConstructionScript`)