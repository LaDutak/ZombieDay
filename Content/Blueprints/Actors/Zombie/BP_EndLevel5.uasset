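; BP_EndLevel5 is a trigger actor that ends level 5 when a BP_Crowd_New actor overlaps it.
; It hides the mouse cursor, waits two seconds so the menu does not appear immediately, then pauses the game.
; It then sets EndLevel on MyPlayerController to launch the menu, shows the cursor, unlocks level 6 in MyGameInstance and records the level number on the controller.
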(event `self.ReceiveActorBeginOverlap`
  (params (OtherActor :type "Actor Object Reference"))
  (cast `/Game/Blueprints/Actors/Crowd/BP_Crowd_New` OtherActor)
  (bind _asmy_player_controller (cast `/Game/Blueprints/AllCharacter/MyPlayerController` (`GameplayStatics.GetPlayerController` 0)))
  ;[1 1 1] Чтобы меню появилось не сразу
  (set `PlayerController.bShowMouseCursor` false _asmy_player_controller)
  (`KismetSystemLibrary.Delay` 2.0)
  (`GameplayStatics.SetGamePaused` true)
  (set `/Game/Blueprints/AllCharacter/MyPlayerController.EndLevel` true _asmy_player_controller) ; Запускает меню
  (set `PlayerController.bShowMouseCursor` true _asmy_player_controller)
  (bind _asmy_game_instance (cast `/Game/Blueprints/AllCharacter/MyGameInstance` (`GameplayStatics.GetGameInstance`)))
  (set `/Game/Blueprints/AllCharacter/MyGameInstance.Is6Opened?` true _asmy_game_instance)
  (set `/Game/Blueprints/AllCharacter/MyPlayerController.NumberOfLevel` 5 _asmy_player_controller))

(fn `UserConstructionScript`)