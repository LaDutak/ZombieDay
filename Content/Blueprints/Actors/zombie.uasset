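; Zombie pawn that can be positioned under the mouse cursor and uses AI to chase the crowd pawn.
; While FollowMouse is set, Tick shows the Plane component and snaps the zombie to the cursor's Visibility hit; otherwise the Plane is hidden.
; Seeing any pawn through PawnSensing sets IsSeeing and calls Follow, which runs AIMoveTo toward the BP_Crowd_Pawn found by GetActorOfClass, whichever pawn was seen.
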(event `self.ReceiveTick`
  (params (DeltaSeconds :type "Float (single-precision)"))
  (bind _plane (`self.Plane`))
  (if (`self.FollowMouse`)
    ;[1 1 1] перемещение под курсором
    (`SceneComponent.SetHiddenInGame` _plane false false)
    (`self.K2_SetActorLocation` (`.Location` (`GameplayStatics.BreakHitResult` (`PlayerController.GetHitResultUnderCursorByChannel` (`GameplayStatics.GetPlayerController` 0) "TraceTypeQuery1" true))))
    (else
      (`SceneComponent.SetHiddenInGame` _plane true false))))

(event `self.PawnSensing.OnSeePawn`
  (params (Pawn :type "Pawn Object Reference"))
  ;[1 1 1] AI
  (cast `/Game/Blueprints/Actors/BP_Crowd_Pawn` Pawn
    (:`then`
      (`KismetSystemLibrary.PrintString` "Hello")
      (set `self.IsSeeing?` true))
    (:`CastFailed`
      (`KismetSystemLibrary.PrintString` "Faild")
      (set `self.IsSeeing?` true)))
  (`self.Follow`))

(event `Follow`
  ;[1 1 1] AI
  (bind _returnvalue (`GameplayStatics.GetActorOfClass` "/Game/Blueprints/Actors/BP_Crowd_Pawn.BP_Crowd_Pawn_C"))
  (`|AIMoveTo` self (0.0 0.0 0.0) _returnvalue 5.0 true))

(fn `UserConstructionScript`)