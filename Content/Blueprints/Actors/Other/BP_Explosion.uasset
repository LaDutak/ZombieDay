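; BP_Explosion is an explosion actor that destroys any BP_Zombie_1 it overlaps.
; When FollowMouse is true, Tick fires a one-time detonation that removes the Cylinder, enlarges the Box, unhides NSExplosion and adds a Niagara component.
; The actor destroys itself after a short delay.
; The overlap kill is not gated on detonation, and nothing in this graph sets FollowMouse.
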(event `self.ReceiveTick`
  (params (DeltaSeconds :type "Float (single-precision)"))
  ;[1 1 1] Курсор и скейл
  (if (`self.FollowMouse`)
    (`/Engine/EditorBlueprintResources/StandardMacros.DoOnce` false
      (:`Completed`
        (`ActorComponent.K2_DestroyComponent` (`self.Cylinder`))
        (`SceneComponent.SetRelativeScale3D` (`self.Box`) (10.0 10.0 10.0))
        (`SceneComponent.SetHiddenInGame` (`self.NS_Explosion`) false false)
        (`AddComponent|NODE_AddNiagaraComponent-0`)
        (`KismetSystemLibrary.Delay` 1.0)
        (`self.K2_DestroyActor`)))))

(event `self.ReceiveActorBeginOverlap`
  (params (OtherActor :type "Actor Object Reference"))
  ;[1 1 1] Смерть врагам
  (bind _asbp_zombie_1 (cast `/Game/Blueprints/Actors/Zombie/BP_Zombie_1` OtherActor))
  (`self.K2_DestroyActor` _asbp_zombie_1))

(fn `UserConstructionScript`)