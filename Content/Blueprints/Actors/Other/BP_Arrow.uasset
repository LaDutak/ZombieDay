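; BP_Arrow is an animated arrow marker that tracks the X and Y position of the Cube1 component on its referenced Crowd.
; A timeline sets its height and ping-pongs through a FlipFlop on finish, so the arrow bobs continuously.
; The construction script feeds Speed into RotatingMovement to spin it.
; Tick destroys the arrow once the Crowd's Counter reaches one or more.
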(event `self.ReceiveTick`
  (params (DeltaSeconds :type "Float (single-precision)"))
  (if (>= (`/Game/Blueprints/Actors/Crowd/BP_Crowd_New.Counter` (`self.Crowd`)) 1)
    (`self.K2_DestroyActor`)))

(event `self.ReceiveBeginPlay`
  (bind (_returnvalue_x _returnvalue_y) (`KismetMathLibrary.BreakVector` (`SceneComponent.GetSocketLocation` (`/Game/Blueprints/Actors/Crowd/BP_Crowd_New.Cube1` (`self.Crowd`)) "None")))
  (bind (_direction _newtrack_0) (`Timeline|Timeline` :!label _label)
    (:`Update`
      (`self.K2_SetActorLocation` (`KismetMathLibrary.MakeVector` _returnvalue_x _returnvalue_y _newtrack_0)))
    (:`Finished`
      (`self.K2_SetActorLocation` (`KismetMathLibrary.MakeVector` _returnvalue_x _returnvalue_y _newtrack_0))
      (`/Engine/EditorBlueprintResources/StandardMacros.FlipFlop`
        (:`A`
          (goto _label :!via `ReverseFromEnd`))
        (:`B`
          (goto _label :!via `PlayFromStart`))))))

(fn `UserConstructionScript`
  (set `RotatingMovementComponent.RotationRate` (`KismetMathLibrary.MakeRotator` 0.0 0.0 (`self.speed`)) (`self.RotatingMovement`)))