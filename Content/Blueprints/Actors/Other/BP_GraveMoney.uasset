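; BP_GraveMoney is a short-lived coin pickup actor that destroys itself five seconds after BeginPlay.
; While its FollowMouse flag is set, Tick advances a counter, then clears both on the second count to register a single click rather than a hold.
; That click adds MoneyPerClick to Coins in MyGameInstance, unhides the NSGraveMoney effect and adds a Niagara component to its owner.
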(event `self.ReceiveTick`
  (params (DeltaSeconds :type "Float (single-precision)"))
  (bind _ns_gravemoney (`self.NS_GraveMoney`))
  ;[1 1 1] Comment
  (if (`self.FollowMouse`)
    (bind _output_get (set `self.Counter` (+ (`self.Counter`) 1)))
    (if (> _output_get 1)
      (set `self.FollowMouse` false)
      (set `self.Counter` 0)
      (bind _asmy_game_instance (cast `/Game/Blueprints/Actors/MyGameInstance` (`GameplayStatics.GetGameInstance`)))
      (set `/Game/Blueprints/Actors/MyGameInstance.Coins` (+ (`/Game/Blueprints/Actors/MyGameInstance.Coins` _asmy_game_instance) (`self.MoneyPerClick`)) _asmy_game_instance)
      (`SceneComponent.SetHiddenInGame` _ns_gravemoney false false)
      (`AddComponent|NODE_AddNiagaraComponent-1` :`self` (`ActorComponent.GetOwner` _ns_gravemoney)))))

(event `self.ReceiveBeginPlay`
  ;[1 1 1] Уничтожение
  (`KismetSystemLibrary.Delay` 5.0)
  (`self.K2_DestroyActor`))

(fn `UserConstructionScript`)