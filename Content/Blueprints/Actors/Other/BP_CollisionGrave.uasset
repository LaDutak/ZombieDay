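; BP_CollisionGrave is a trigger actor that animates and removes a referenced Grave when a BP_Crowd_New actor overlaps it.
; A timeline drives the Grave's world Z, and its update also reveals the Grave's Niagara effect, prints debug text and destroys the Grave after a delay.
; An unconnected branch holds a similar timed move-and-destroy sequence gated on the Grave's ConterMoney count.
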(event `self.ReceiveActorBeginOverlap`
  (params (OtherActor :type "Actor Object Reference"))
  (bind _grave (`self.Grave`))
  (bind _defaultsceneroot (`/Game/Blueprints/Actors/Other/BP_GraveMoney.DefaultSceneRoot` _grave))
  (bind (_returnvalue_x _returnvalue_y) (`KismetMathLibrary.BreakVector` (`SceneComponent.K2_GetComponentLocation` _defaultsceneroot)))
  (bind _asbp_crowd_new (cast `/Game/Blueprints/Actors/Crowd/BP_Crowd_New` OtherActor))
  (`/Engine/EditorBlueprintResources/StandardMacros.IsValid` _asbp_crowd_new
    (:`Is Valid`
      (bind (_direction _newtrack_0) (`Timeline|Timeline`)
        (:`Update`
          (`SceneComponent.K2_SetWorldLocation` _defaultsceneroot (`KismetMathLibrary.MakeVector` _returnvalue_x _returnvalue_y _newtrack_0) false false)
          (`SceneComponent.SetHiddenInGame` (`/Game/Blueprints/Actors/Other/BP_GraveMoney.Niagara` _grave) false false)
          (`KismetSystemLibrary.PrintString` "Hello")
          (`KismetSystemLibrary.Delay` 5.0)
          (`self.K2_DestroyActor` _grave))))))

(fn `UserConstructionScript`)