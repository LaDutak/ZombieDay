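; BP_Train1 is a train actor that runs its Cube along a spline and destroys BP_Zombie_1 actors that overlap it.
; While FollowMouse is set, Tick advances the Cube a fixed, frame-rate-dependent step along the spline.
; An unchanged position signals the end: the Cube hides, resets its distance after a delay, reappears and clears FollowMouse.
; The second overlap cast, to test, only runs after the zombie cast succeeds.
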(event `self.ReceiveTick`
  (params (DeltaSeconds :type "Float (single-precision)"))
  (if (`self.FollowMouse`)
    (`self.CustomEvent`)))

(event `self.ReceiveBeginPlay`)

(event `CustomEvent`
  (bind _cube (`self.Cube`))
  (bind _cube_2 (`self.Cube`))
  (bind (_returnvalue_location _returnvalue_rotation) (`KismetMathLibrary.BreakTransform` (`SplineComponent.GetTransformAtDistanceAlongSpline` (`self.Spline`) (`self.Distance`) "Local" false)))
  ;[1 1 1] Перемещение по сплайну
  (set `self.IsFinished?` false)
  (set `self.Distance` (+ (`self.Distance`) 30.0))
  (`SceneComponent.K2_SetRelativeTransform` _cube (`KismetMathLibrary.MakeTransform` _returnvalue_location _returnvalue_rotation (`SceneComponent.RelativeScale3D` _cube)) false false) ; толпа
  (bind _output_get (set `self.Location of Crowd` (`SceneComponent.RelativeLocation` _cube)))
  (if (== _output_get (`self.Distance_Start`))
    (`SceneComponent.SetHiddenInGame` _cube_2 true false)
    (`KismetSystemLibrary.Delay` 3.0)
    (set `self.Distance` 0.0)
    (`KismetSystemLibrary.Delay` 0.1)
    (`SceneComponent.SetHiddenInGame` _cube_2 false false)
    (set `self.IsFinished?` true)
    (set `self.FollowMouse` false)
    (else
      (set `self.Distance_Start` _output_get))))

(event `self.ReceiveActorBeginOverlap`
  (params (OtherActor :type "Actor Object Reference"))
  ;[1 1 1] Смерть всем
  (bind _asbp_zombie_1 (cast `/Game/Blueprints/Actors/Zombie/BP_Zombie_1` OtherActor))
  (`self.K2_DestroyActor` _asbp_zombie_1)
  (bind _astest (cast `/Game/Blueprints/Actors/Crowd/test` OtherActor))
  (`self.K2_DestroyActor` _astest))

(fn `UserConstructionScript`)