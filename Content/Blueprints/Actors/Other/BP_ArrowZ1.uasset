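; BP_ArrowZ1 is a spinning, bobbing arrow marker that hovers at BP_Killer's position while BP_Zombie_1 is following the mouse.
; Tick shows the Cube only while Collision.Spawned and the zombie's FollowMouse are true, and otherwise hides it.
; A Timeline copies X/Y from the killer's Box and drives Z, with a FlipFlop alternating reverse and forward playback.
; The construction script sets the RotatingMovement rate from Speed.
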(event `self.ReceiveBeginPlay`)

(event `self.ReceiveTick`
  (params (DeltaSeconds :type "Float (single-precision)"))
  (bind _cube (`self.Cube`))
  (if (`/Game/Blueprints/Actors/Other/BP_CollisionSpawn.Spawned` (`self.Collision`))
    (if (`/Game/Blueprints/Actors/Zombie/BP_Zombie_1.FollowMouse` (stale _returnvalue))
      (`SceneComponent.SetHiddenInGame` _cube false false)
      (bind _returnvalue (`GameplayStatics.GetActorOfClass` "/Game/Blueprints/Actors/Zombie/BP_Zombie_1.BP_Zombie_1_C"))
      (bind (_direction _newtrack_0) (`Timeline|Timeline` :!label _label)
        (:`Update`
          (bind _returnvalue_2 (`GameplayStatics.GetActorOfClass` "/Game/Blueprints/Actors/Zombie/BP_Killer.BP_Killer_C"))
          (bind (_returnvalue_x _returnvalue_y) (`KismetMathLibrary.BreakVector` (`SceneComponent.GetSocketLocation` (`/Game/Blueprints/Actors/Zombie/BP_Killer.Box` _returnvalue_2) "None")))
          (`self.K2_SetActorLocation` (`KismetMathLibrary.MakeVector` _returnvalue_x _returnvalue_y _newtrack_0)))
        (:`Finished`
          (bind _returnvalue_3 (`GameplayStatics.GetActorOfClass` "/Game/Blueprints/Actors/Zombie/BP_Killer.BP_Killer_C"))
          (bind (_returnvalue_x_2 _returnvalue_y_2) (`KismetMathLibrary.BreakVector` (`SceneComponent.GetSocketLocation` (`/Game/Blueprints/Actors/Zombie/BP_Killer.Box` _returnvalue_3) "None")))
          (`self.K2_SetActorLocation` (`KismetMathLibrary.MakeVector` _returnvalue_x_2 _returnvalue_y_2 _newtrack_0))
          (`/Engine/EditorBlueprintResources/StandardMacros.FlipFlop`
            (:`A`
              (goto _label :!via `ReverseFromEnd`))
            (:`B`
              (goto _label :!via `PlayFromStart`)))))
      (else
        (`SceneComponent.SetHiddenInGame` _cube true false)))
    (else
      (`KismetSystemLibrary.PrintString` "aaaa")
      (`SceneComponent.SetHiddenInGame` _cube true false))))

(fn `UserConstructionScript`
  (set `RotatingMovementComponent.RotationRate` (`KismetMathLibrary.MakeRotator` 0.0 0.0 (`self.speed`)) (`self.RotatingMovement`)))