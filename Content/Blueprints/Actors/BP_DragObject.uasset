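; BP_DragObject is a draggable actor that follows the mouse cursor while its FollowMouse flag is set.
; Each Tick it moves, without sweeping, to the hit location of a complex visibility trace under player 0's cursor.
; Its PawnSensing and Follow events are empty; leftover logic for spotting pawns and AI-moving to BP_Crowd_Pawn is disconnected and never runs.
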(event `self.ReceiveTick`
  (params (DeltaSeconds :type "Float (single-precision)"))
  ;[1 1 1] перемещение под курсором
  (if (`self.FollowMouse`)
    (`self.K2_SetActorLocation` (`.Location` (`GameplayStatics.BreakHitResult` (`PlayerController.GetHitResultUnderCursorByChannel` (`GameplayStatics.GetPlayerController` 0) "TraceTypeQuery1" true))))))

(event `self.PawnSensing.OnSeePawn`
  (params (Pawn :type "Pawn Object Reference")))

(event `Follow`)

(fn `UserConstructionScript`)