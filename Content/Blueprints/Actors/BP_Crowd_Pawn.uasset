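; Crowd pawn that steps its Cube along a Spline when flagged by FollowMouse, which the comments tie to a cursor click on the object.
; Tick counts frames while the flag is set, then on the second clears flag and counter, intended to register a click rather than a hold.
; It then advances Distance by a fixed step and applies the spline's local location and rotation to the Cube, keeping its scale.
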(event `self.ReceiveTick`
  (params (DeltaSeconds :type "Float (single-precision)"))
  (bind (_returnvalue_location _returnvalue_rotation) (`KismetMathLibrary.BreakTransform` (`SplineComponent.GetTransformAtDistanceAlongSpline` (`self.Spline`) (`self.Distance`) "Local" false)))
  ;[1 1 1] Клик курсором
  (if (`self.FollowMouse`)
    (bind _output_get (set `self.Counter` (+ (`self.Counter`) 1)))
    (if (> _output_get 1)
      (set `self.FollowMouse` false)
      (set `self.Counter` 0)
      ;[1 1 1] Перемещение по сплайну
      (set `self.Distance` (+ (`self.Distance`) 30.0))
      (`SceneComponent.K2_SetRelativeTransform` (`self.Cube`) (`KismetMathLibrary.MakeTransform` _returnvalue_location _returnvalue_rotation (`SceneComponent.RelativeScale3D` (`self.Cube`))) false false))))

(fn `UserConstructionScript`)