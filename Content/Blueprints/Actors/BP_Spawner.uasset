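; BP_Spawner is an actor that periodically spawns a Zombie above its Cube component and destroys actors that overlap it.
; Tick accumulates a timer and, every five seconds, force-spawns the Zombie regardless of collision and prints a debug string.
; Each spawn raises the Undestoyadle flag, which a Delay clears three seconds later, so overlapping actors are destroyed only outside that grace window.
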(event `self.ReceiveActorBeginOverlap`
  (params (OtherActor :type "Actor Object Reference"))
  (if (not (`self.Undestoyadle?`))
    (`self.K2_DestroyActor` OtherActor)))

(event `self.ReceiveTick`
  (params (DeltaSeconds :type "Float (single-precision)"))
  (bind (_returnvalue_x _returnvalue_y _returnvalue_z) (`KismetMathLibrary.BreakVector` (`SceneComponent.K2_GetComponentLocation` (`self.Cube`))))
  (bind _output_get (set `self.Timer` (+ DeltaSeconds (`self.Timer`))))
  (if (>= _output_get 5.0)
    (set `self.Undestoyadle?` true)
    (`|SpawnActorFromClass` "/Game/Blueprints/Actors/zombie.zombie_C" (`KismetMathLibrary.MakeTransform` (`KismetMathLibrary.MakeVector` _returnvalue_x _returnvalue_y (+ _returnvalue_z 200.0))) "AlwaysSpawn" "MultiplyWithRoot" null null)
    (`KismetSystemLibrary.PrintString` "Hello")
    (set `self.Timer` 0.0)
    (`KismetSystemLibrary.Delay` 3.0)
    (set `self.Undestoyadle?` false)))

(fn `UserConstructionScript`)