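; Player controller that turns on the mouse cursor and touch events when play begins.
; Every tick it casts the game instance to MyGameInstance and prints its coin count, followed by unlock flags for the second, third and fourth levels, as debug strings.
; It contains no other input or gameplay logic, and its construction script is empty.
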(event `self.ReceiveBeginPlay`
  ;[1 1 1] Cursor
  (set `self.bShowMouseCursor` true)
  (set `self.bEnableTouchEvents` true))

(event `self.ReceiveTick`
  (params (DeltaSeconds :type "Float (single-precision)"))
  (bind _asnew_blueprint_2 (cast `/Game/Blueprints/Actors/MyGameInstance` (`GameplayStatics.GetGameInstance`)))
  (`KismetSystemLibrary.PrintString` (`KismetStringLibrary.Conv_IntToString` (`/Game/Blueprints/Actors/MyGameInstance.Coins` _asnew_blueprint_2)) true true (struct :`G` 0.66 :`B` 1.0 :`A` 1.0) 0.0)
  (`KismetSystemLibrary.PrintString` (`KismetStringLibrary.Conv_BoolToString` (`self.IsSecondLevelOpend?`)) true true (struct :`G` 0.66 :`B` 1.0 :`A` 1.0) 0.0)
  (`KismetSystemLibrary.PrintString` (`KismetStringLibrary.Conv_BoolToString` (`self.IsThirdLevelOpend?`)) true true (struct :`G` 0.66 :`B` 1.0 :`A` 1.0) 0.0)
  (`KismetSystemLibrary.PrintString` (`KismetStringLibrary.Conv_BoolToString` (`self.Is4LevelOpend?`)) true true (struct :`G` 0.66 :`B` 1.0 :`A` 1.0) 0.0))

(fn `UserConstructionScript`)