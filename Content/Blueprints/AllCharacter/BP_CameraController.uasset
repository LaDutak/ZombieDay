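; Camera controller that handles swipe panning and press-and-drag of trains, money graves, explosion actors, zombies, crowds and walls.
; Each DragCamera press handler traces under the cursor, casts to one type and sets FollowMouse until release; trains require IsFinished, crowds not DontTouch.
; Tick offsets the camera by the mouse delta while left mouse is held.
; Only dragging BP_Zombie_1 blocks panning, until a short delay after release.
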(event `InputAction|DragCamera`
  (params (Key :type "Key Structure"))
  (bind _as_bp_train_1 (`self.As BP Train 1`))
  ;[1 1 1] Движение по касанию
  ;;[1 1 1] поезда
  (:`Pressed`
    ;;;[1 1 1] Для движения пальцем
    (bind _returnvalue (`WidgetLayoutLibrary.GetMousePositionOnViewport`))
    (set `self.PreviousTouchLocation` _returnvalue)
    (bind _asbp_train_b (cast `/Game/Blueprints/Actors/Other/BP_TrainB` (`.HitActor` (`GameplayStatics.BreakHitResult` (`PlayerController.GetHitResultUnderCursorByChannel` (`GameplayStatics.GetPlayerController` 0) "TraceTypeQuery3" true)))))
    (if (`/Game/Blueprints/Actors/Other/BP_TrainB.IsFinished?` _asbp_train_b)
      (set `/Game/Blueprints/Actors/Other/BP_TrainB.FollowMouse` true _asbp_train_b)
      (set `self.As BP Train 1` _asbp_train_b)))
  (:`Released`
    (`/Engine/EditorBlueprintResources/StandardMacros.IsValid` _as_bp_train_1
      (:`Is Valid`
        (set `/Game/Blueprints/Actors/Other/BP_TrainB.FollowMouse` false _as_bp_train_1)))))

(event `InputAction|DragCamera`
  (params (Key :type "Key Structure"))
  (bind _as_bp_grave_money (`self.As BP Grave Money`))
  ;[1 1 1] Движение по касанию
  ;;[1 1 1] могила с деньгами
  (:`Pressed`
    ;;;[1 1 1] Для движения пальцем
    (bind _returnvalue (`WidgetLayoutLibrary.GetMousePositionOnViewport`))
    (set `self.PreviousTouchLocation` _returnvalue)
    (bind _asbp_grave_money (cast `/Game/Blueprints/Actors/Other/BP_GraveMoney` (`.HitActor` (`GameplayStatics.BreakHitResult` (`PlayerController.GetHitResultUnderCursorByChannel` (`GameplayStatics.GetPlayerController` 0) "TraceTypeQuery3" true)))))
    (set `/Game/Blueprints/Actors/Other/BP_GraveMoney.FollowMouse` true _asbp_grave_money)
    (set `self.As BP Grave Money` _asbp_grave_money))
  (:`Released`
    (`/Engine/EditorBlueprintResources/StandardMacros.IsValid` _as_bp_grave_money
      (:`Is Valid`
        (set `/Game/Blueprints/Actors/Other/BP_GraveMoney.FollowMouse` false _as_bp_grave_money)))))

(event `InputAction|DragCamera`
  (params (Key :type "Key Structure"))
  (bind _as_bp_explosion (`self.As BP Explosion`))
  ;[1 1 1] Движение по касанию
  ;;[1 1 1] Определение бочки
  (:`Pressed`
    ;;;[1 1 1] Для движения пальцем
    (bind _returnvalue (`WidgetLayoutLibrary.GetMousePositionOnViewport`))
    (set `self.PreviousTouchLocation` _returnvalue)
    (bind _asbp_explosion (cast `/Game/Blueprints/Actors/Other/BP_Explosion` (`.HitActor` (`GameplayStatics.BreakHitResult` (`PlayerController.GetHitResultUnderCursorByChannel` (`GameplayStatics.GetPlayerController` 0) "TraceTypeQuery3" true)))))
    (set `/Game/Blueprints/Actors/Other/BP_Explosion.FollowMouse` true _asbp_explosion)
    (set `self.As BP Explosion` _asbp_explosion))
  (:`Released`
    (`/Engine/EditorBlueprintResources/StandardMacros.IsValid` _as_bp_explosion
      (:`Is Valid`
        (set `/Game/Blueprints/Actors/Other/BP_Explosion.FollowMouse` false _as_bp_explosion)))))

(event `self.ReceiveTick`
  (params (DeltaSeconds :type "Float (single-precision)"))
  (bind _returnvalue (`WidgetLayoutLibrary.GetViewportScale`))
  (bind _as_zombie (`self.As Zombie`))
  (bind (_returnvalue_x _returnvalue_y) (`KismetMathLibrary.BreakVector2D` (- (`self.NewTouchLocation`) (`self.PreviousTouchLocation`))))
  (bind (_x _y) (`KismetMathLibrary.BreakVector2D` (- (* (0.0 0.0) (`KismetMathLibrary.MakeVector2D` _returnvalue _returnvalue)) (/ (`WidgetLayoutLibrary.GetViewportSize`) (2.0 2.0)))))
  ;[1 1 1] Движение по касанию
  ;;[1 1 1] Переджижение с зажатым зомби
  (`/Engine/EditorBlueprintResources/StandardMacros.IsValid` _as_zombie
    (:`Is Valid`
      (if (`/Game/Blueprints/Actors/Zombie/BP_Zombie_1.FollowMouse` _as_zombie)
        (set `self.DoNotMove` true)
        (else
          (if (`self.DoNotMove`) :!label _label
            (`KismetSystemLibrary.Delay` 0.4)
            (set `self.DoNotMove` false)
            (else
              ;;[1 1 1] Свайп пальцем
              (set `self.Alpha` 0.0)
              (bind _returnvalue_2 (`WidgetLayoutLibrary.GetMousePositionOnViewport`))
              (if (`PlayerController.IsInputKeyDown` (`GameplayStatics.GetPlayerController` 0) "LeftMouseButton")
                (set `self.NewTouchLocation` _returnvalue_2)
                (`SceneComponent.K2_AddWorldOffset` (`self.Camera`) (`KismetMathLibrary.MakeVector` _returnvalue_y (* _returnvalue_x -1.0)) false false)
                (set `self.PreviousTouchLocation` (`self.NewTouchLocation`))
                (set `self.NewVar_0` (+ (* (`KismetMathLibrary.GreaterGreater_VectorRotator` (`KismetMathLibrary.MakeVector` _x _y) (struct :`Yaw` 90.0)) (`self.NewVar`)) (`self.K2_GetActorLocation`)))))))))
    (:`Is Not Valid`
      (goto _label))))

(event `InputAction|DragCamera`
  (params (Key :type "Key Structure"))
  (bind _as_zombie (`self.As Zombie`))
  ;[1 1 1] Движение по касанию
  ;;[1 1 1] Перемещение под кусросром для AI
  (:`Pressed`
    ;;;[1 0 0.1969] Для движения пальцем
    (bind _returnvalue (`WidgetLayoutLibrary.GetMousePositionOnViewport`))
    (set `self.PreviousTouchLocation` _returnvalue)
    (bind _asbp_zombie_1 (cast `/Game/Blueprints/Actors/Zombie/BP_Zombie_1` (`.HitActor` (`GameplayStatics.BreakHitResult` (`PlayerController.GetHitResultUnderCursorByChannel` (`GameplayStatics.GetPlayerController` 0) "TraceTypeQuery3" true)))))
    (set `/Game/Blueprints/Actors/Zombie/BP_Zombie_1.FollowMouse` true _asbp_zombie_1)
    (set `self.As Zombie` _asbp_zombie_1))
  (:`Released`
    (`/Engine/EditorBlueprintResources/StandardMacros.IsValid` _as_zombie
      (:`Is Valid`
        (set `/Game/Blueprints/Actors/Zombie/BP_Zombie_1.FollowMouse` false _as_zombie)))))

(event `InputAction|DragCamera`
  (params (Key :type "Key Structure"))
  (bind _as_test (`self.As Test`))
  ;[1 1 1] Движение по касанию
  (:`Pressed`
    ;;[1 1 1] Толпа
    ;;;[1 1 1] Для движения пальцем
    (bind _returnvalue (`WidgetLayoutLibrary.GetMousePositionOnViewport`))
    (set `self.PreviousTouchLocation` _returnvalue)
    (bind _asbp_crowd_new (cast `/Game/Blueprints/Actors/Crowd/BP_Crowd_New` (`.HitActor` (`GameplayStatics.BreakHitResult` (`PlayerController.GetHitResultUnderCursorByChannel` (`GameplayStatics.GetPlayerController` 0) "TraceTypeQuery3" true)))))
    (if (not (`/Game/Blueprints/Actors/Crowd/BP_Crowd_New.Don't Touch` _asbp_crowd_new))
      (set `/Game/Blueprints/Actors/Crowd/BP_Crowd_New.FollowMouse` true _asbp_crowd_new)
      (set `self.As Test` _asbp_crowd_new)))
  (:`Released`
    (`/Engine/EditorBlueprintResources/StandardMacros.IsValid` _as_test
      (:`Is Valid`
        (if (not (`/Game/Blueprints/Actors/Crowd/BP_Crowd_New.Don't Touch` _as_test))
          (set `/Game/Blueprints/Actors/Crowd/BP_Crowd_New.FollowMouse` false _as_test))))))

(event `InputAction|DragCamera`
  (params (Key :type "Key Structure"))
  (bind _as_bp_zombie_2 (`self.As BP Zombie 2`))
  ;[1 1 1] Движение по касанию
  ;;[1 1 1] Перемещение под кусросром для AI
  (:`Pressed`
    ;;;[1 0 0.1969] Для движения пальцем
    (bind _returnvalue (`WidgetLayoutLibrary.GetMousePositionOnViewport`))
    (set `self.PreviousTouchLocation` _returnvalue)
    (bind _asbp_zombie_2 (cast `/Game/Blueprints/Actors/Zombie/BP_Zombie_2` (`.HitActor` (`GameplayStatics.BreakHitResult` (`PlayerController.GetHitResultUnderCursorByChannel` (`GameplayStatics.GetPlayerController` 0) "TraceTypeQuery3" true)))))
    (set `/Game/Blueprints/Actors/Zombie/BP_Zombie_2.FollowMouse` true _asbp_zombie_2)
    (set `self.As BP Zombie 2` _asbp_zombie_2))
  (:`Released`
    (`/Engine/EditorBlueprintResources/StandardMacros.IsValid` _as_bp_zombie_2
      (:`Is Valid`
        (set `/Game/Blueprints/Actors/Zombie/BP_Zombie_2.FollowMouse` false _as_bp_zombie_2)))))

(event `InputAction|DragCamera`
  (params (Key :type "Key Structure"))
  (bind _as_bp_wall (`self.As BP Wall`))
  ;[1 1 1] Движение по касанию
  ;;[1 1 1] Дверь
  (:`Pressed`
    ;;;[1 1 1] Для движения пальцем
    (bind _returnvalue (`WidgetLayoutLibrary.GetMousePositionOnViewport`))
    (set `self.PreviousTouchLocation` _returnvalue)
    (bind _asbp_wall (cast `/Game/Blueprints/Actors/Other/BP_Wall` (`.HitActor` (`GameplayStatics.BreakHitResult` (`PlayerController.GetHitResultUnderCursorByChannel` (`GameplayStatics.GetPlayerController` 0) "TraceTypeQuery3" true)))))
    (set `/Game/Blueprints/Actors/Other/BP_Wall.FollowMouse` true _asbp_wall)
    (set `self.As BP Wall` _asbp_wall))
  (:`Released`
    (`/Engine/EditorBlueprintResources/StandardMacros.IsValid` _as_bp_wall
      (:`Is Valid`
        (set `/Game/Blueprints/Actors/Other/BP_Wall.FollowMouse` false _as_bp_wall)))))

(fn `UserConstructionScript`)